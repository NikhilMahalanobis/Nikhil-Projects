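; MenuCharacterComponent is an actor component that owns the character's pause menu and toggles it on screen.
; InitializeMenu stores the player controller and creates a MenuContainer widget for it once, without displaying it.
; OpenPauseMenuKeyboard flips IsOpen, adding that widget to the viewport with Game and UI input mode focused on it, or removing it.
; Closing leaves the input mode unchanged.
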(event EventBeginPlay)

(event EventTick
  (params (DeltaSeconds :type Float%20%28single-precision%29)))

(fn InitializeMenu
  (params (Player%20Controller :type Player%20Controller%20Object%20Reference%20%28by%20ref%29))
  (bind _output_get (Variables|Default|SetPlayer%20Controlelr Player%20Controller))
  (bind _returnvalue (UserInterface|CreateWidget "/Game/Blueprints/PauseMenu/MenuWidgets/MenuContainer.MenuContainer_C" _output_get))
  (Variables|Default|SetMenu _returnvalue))

(fn OpenPauseMenuKeyboard
  (bind _menu (Variables|Default|GetMenu))
  (if (Variables|Default|GetIsOpen)
    (Widget|RemovefromParent (Variables|Default|GetMenu))
    (Variables|Default|SetIsOpen false)
    (else
      (UserInterface|Viewport|AddtoViewport _menu 0)
      (Input|SetInputModeGameandUI (Variables|Default|GetPlayer%20Controlelr) _menu "DoNotLock" false)
      (Variables|Default|SetIsOpen true))))